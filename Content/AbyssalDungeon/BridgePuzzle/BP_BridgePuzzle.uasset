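; Bridge puzzle actor that rotates three bridge components and signals a wall to open once their rotations match the solution.
; An overlap box enables input and the interact prompt; E calls TryRotate for all four indices, but the IsMoving guard admits only the first.
; Tick interpolates each bridge by its indexed offset, then disables itself, saves new start rotations and compares them against CompleteRotations within a tolerance.
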(event OnComponentBeginOverlap(Box)
  (params (OverlappedComponent :type Primitive%20Component%20Object%20Reference) (OtherActor :type Actor%20Object%20Reference) (OtherComp :type Primitive%20Component%20Object%20Reference) (OtherBodyIndex :type Integer) (bFromSweep :type Boolean) (SweepResult :type Hit%20Result%20Structure%20%28by%20ref%29))
  (Utilities|Casting|CastToBP_FirstPersonCharacter OtherActor)
  (Input|EnableInput (Game|GetPlayerController 0))
  (if (== OtherActor (Game|GetPlayerCharacter 0))
    (UserInterface|Viewport|AddtoViewport (Variables|Default|GetInteractPrompt) 0)))

(event OnComponentEndOverlap(Box)
  (params (OverlappedComponent :type Primitive%20Component%20Object%20Reference) (OtherActor :type Actor%20Object%20Reference) (OtherComp :type Primitive%20Component%20Object%20Reference) (OtherBodyIndex :type Integer))
  (Utilities|Casting|CastToBP_FirstPersonCharacter OtherActor)
  (Input|DisableInput (Game|GetPlayerController 0))
  (if (== (Game|GetPlayerCharacter 0) OtherActor)
    (Widget|RemovefromParent (Variables|Default|GetInteractPrompt))))

(event Custom|RotateBridge
  (for _array_element (Variables|Default|GetData)
    (Transformation|SetRelativeRotation (.Component (Utilities|Struct|BreakS_BridgePuzzleData _array_element)) (Math|Rotator|CombineRotators (.StartRotation (Utilities|Struct|BreakS_BridgePuzzleData _array_element)) (Math|Rotator|MakeRotator (* (.roll (Utilities|Array|Get(acopy) (.Rotation (Utilities|Struct|BreakS_BridgePuzzleData _array_element)) (Variables|Default|GetRotationIndex))) (/ (Variables|Default|GetCurrentTime) (Variables|Default|GetRotationTime))) (* (.pitch (Utilities|Array|Get(acopy) (.Rotation (Utilities|Struct|BreakS_BridgePuzzleData _array_element)) (Variables|Default|GetRotationIndex))) (/ (Variables|Default|GetCurrentTime) (Variables|Default|GetRotationTime))) (* (.yaw (Utilities|Array|Get(acopy) (.Rotation (Utilities|Struct|BreakS_BridgePuzzleData _array_element)) (Variables|Default|GetRotationIndex))) (/ (Variables|Default|GetCurrentTime) (Variables|Default|GetRotationTime))))) false false))
  (if (>= (Variables|Default|GetCurrentTime) (Variables|Default|GetRotationTime))
    (Variables|Default|SetIsMoving? false)
    (Actor|Tick|SetActorTickEnabled false)
    (Variables|Default|SetCurrentTime 0.0)
    (for (_array_element_2 _array_index) (Variables|Default|GetData)
      (Transformation|SetRelativeRotation (.Component (Utilities|Struct|BreakS_BridgePuzzleData _array_element_2)) (Math|Rotator|CombineRotators (.StartRotation (Utilities|Struct|BreakS_BridgePuzzleData _array_element_2)) (Utilities|Array|Get(acopy) (.Rotation (Utilities|Struct|BreakS_BridgePuzzleData _array_element_2)) (Variables|Default|GetRotationIndex))) false false)
      (bind _structout (Utilities|Struct|SetmembersinS_BridgePuzzleData _array_element_2 (Math|Rotator|CombineRotators (.StartRotation (Utilities|Struct|BreakS_BridgePuzzleData _array_element_2)) (Utilities|Array|Get(acopy) (.Rotation (Utilities|Struct|BreakS_BridgePuzzleData _array_element_2)) (Variables|Default|GetRotationIndex)))))
      (Utilities|Array|SetArrayElem (Variables|Default|GetData) _array_index _structout))
    (bind _success (CallFunction|IsPuzzleFinished))
    (if _success
      (Class|BPIBridgePuzzle|OpenWall(Message) (Variables|Default|GetWall)))))

(event Custom|TryRotate
  (params (RotationIndex :type Integer))
  (if (not (Variables|Default|GetIsMoving?))
    (Variables|Default|SetIsMoving? true)
    (Variables|Default|SetRotationIndex RotationIndex)
    (Actor|Tick|SetActorTickEnabled true)))

(event EventTick
  (params (DeltaSeconds :type Float%20%28single-precision%29))
  (Variables|Default|SetCurrentTime (+ DeltaSeconds (Variables|Default|GetCurrentTime)))
  (CallFunction|RotateBridge))

(event EventBeginPlay
  (bind _bridge2 (Variables|Default|GetBridge2))
  (bind _bridge3 (Variables|Default|GetBridge3))
  (bind _bridge1 (Variables|Default|GetBridge1))
  (Utilities|Array|Add (Variables|Default|GetData) (Utilities|Struct|MakeS_BridgePuzzleData _bridge1 (Variables|/Script/Engine.SceneComponent|GetRelativeRotation _bridge1) (Utilities|Array|MakeArray "10.000000,0.000000,0.000000" "25.000000,0.000000,0.000000" "-30.000000,0.000000,0.000000" "-15.000000,0.000000,0.000000")))
  (Utilities|Array|Add (Variables|Default|GetData) (Utilities|Struct|MakeS_BridgePuzzleData _bridge2 (Variables|/Script/Engine.SceneComponent|GetRelativeRotation _bridge2) (Utilities|Array|MakeArray "40.000000,0.000000,0.000000" "15.000000,0.000000,0.000000" "-10.000000,0.000000,0.000000" "-25.000000,0.000000,0.000000")))
  (Utilities|Array|Add (Variables|Default|GetData) (Utilities|Struct|MakeS_BridgePuzzleData _bridge3 (Variables|/Script/Engine.SceneComponent|GetRelativeRotation _bridge3) (Utilities|Array|MakeArray "35.000000,0.000000,0.000000" "25.000000,0.000000,0.000000" "-15.000000,0.000000,0.000000" "-5.000000,0.000000,0.000000")))
  (bind _returnvalue (UserInterface|CreateWidget "/Game/AbyssalDungeon/UI/WB_InteractPromptBridge.WB_InteractPromptBridge_C"))
  (Variables|Default|SetInteractPrompt _returnvalue))

(event Input|KeyboardEvents|4
  (params (Key :type Key%20Structure :default "None")))

(event Input|KeyboardEvents|E
  (params (Key :type Key%20Structure :default "None"))
  (:Pressed
    (Utilities|FlowControl|Sequence
      (:then_0
        (CallFunction|TryRotate))
      (:then_1
        (CallFunction|TryRotate 1))
      (:then_2
        (CallFunction|TryRotate 2))
      (:then_3
        (CallFunction|TryRotate 3)))))

(event Input|KeyboardEvents|2
  (params (Key :type Key%20Structure :default "None")))

(event Input|KeyboardEvents|3
  (params (Key :type Key%20Structure :default "None")))

(fn ConstructionScript)

(fn IsPuzzleFinished
  (for (_array_element _array_index) (Variables|Default|GetCompleteRotations)
    (if (not (Utilities|Operators|EqualEqual (Variables|/Script/Engine.SceneComponent|GetRelativeRotation (.component (Utilities|Array|Get(acopy) (Variables|Default|GetData) _array_index))) _array_element 0.5))
      (LocalVariables|SetL_Success false)))
  (return (LocalVariables|GetL_Success)))