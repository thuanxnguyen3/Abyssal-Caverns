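; BP_MoveableWall2 is a puzzle wall in the Abyssal Dungeon bridge puzzle that moves vertically when enough pressure switches are active.
; SwitchActivated and SwitchDeactivated events adjust an active switch count and compare it to the required number.
; Meeting the threshold plays the DoorActivation timeline, which drives the wall's relative Z location, and falling below it reverses the timeline.
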(event Custom|SwitchActivated
  (Math|Integer|IncrementInt (Variables|Default|GetPressureSwitchActive)
    (:%20%20
      (if (>= (Variables|Default|GetPressureSwitchActive) (Variables|Default|GetPressureSwitchNeeded))
        (bind _doorposition (Timeline|DoorActivation Play)
          (:Update
            (Transformation|SetRelativeLocation (Variables|Default|GetWall) (Math|Vector|MakeVector 0.0 0.0 _doorposition) false false)))
        (else
          (Timeline|DoorActivation Reverse))))))

(event Custom|SwitchDeactivated
  (Math|Integer|DecrementInt (Variables|Default|GetPressureSwitchActive)
    (:%20%20
      (if (>= (Variables|Default|GetPressureSwitchActive) (Variables|Default|GetPressureSwitchNeeded))
        (bind _doorposition (Timeline|DoorActivation Play)
          (:Update
            (Transformation|SetRelativeLocation (Variables|Default|GetWall) (Math|Vector|MakeVector 0.0 0.0 _doorposition) false false)))
        (else
          (Timeline|DoorActivation Reverse))))))

(fn ConstructionScript)